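; Quest manager actor that registers quests, tracks the selected one and guides the player to its current sub-goal.
; AddNewQuest spawns each quest class once and lists it in the main widget, auto-selecting it through SelectNewQuest when requested or first.
; Switching sub-goals respawns a goal actor for located objectives.
; Player movement updates horizontal distance in metres and the minimap arrow, with paired DoOnce nodes toggling arrow visibility around a distance threshold.
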(event Custom|OnSwitchSubQuest
  (bind _currentquest (Variables|Default|GetCurrentQuest))
  (bind _mainwidget (Variables|Default|GetMainWidget))
  (Utilities|IsValid (Variables|Default|GetCurrentGoalActor)
    (:Is%20Valid
      (Actor|DestroyActor (Variables|Default|GetCurrentGoalActor)))
    (:Is%20Not%20Valid
      _))
  (bind _output_get (Variables|Default|SetCurrentSubGoal (Utilities|Array|Get(acopy) (.SubGoal (Utilities|Struct|BreakS_QuestInfo (Variables|/Game/Blueprints/Actors/QuestActors/BP_MasterQuest.BP_MasterQuest_C|GetQuestInfo _currentquest))) (Variables|/Game/Blueprints/Actors/QuestActors/BP_MasterQuest.BP_MasterQuest_C|GetSelectedSubGoalIndex _currentquest))))
  (if (.hasLocation (Utilities|Struct|BreakS_GoalLocation (.GoalLocation (Utilities|Struct|BreakS_GoalInfo _output_get))))
    (bind _returnvalue (Game|SpawnActorfromClass "/Game/Blueprints/Actors/BP_GoalActor.BP_GoalActor_C" (Math|Transform|MakeTransform (.Locaion (Utilities|Struct|BreakS_GoalLocation (.GoalLocation (Utilities|Struct|BreakS_GoalInfo _output_get)))) "0, 0, 0" "1,1,1") "AlwaysSpawn" 0 0))
    (Variables|Default|SetCurrentGoalActor _returnvalue)
    (bind _output_get_2 (Variables|Default|SetCurrentDistance (CallFunction|DistancetoGoal)))
    (Rendering|Components|TextRender|SetText (Variables|/Game/Widget/HUDWidget.HUDWidget_C|GetDistanceText (Variables|Default|GetMainWidget)) (Utilities|Text|ToText(Integer) _output_get_2 false false))
    (CallFunction|UpdateDirectionArrow)
    (Widget|SetVisibility (Variables|/Game/Widget/HUDWidget.HUDWidget_C|GetDistanceBorder _mainwidget) "HitTestInvisible")
    (Widget|SetVisibility (Variables|/Game/Widget/MiniMap.MiniMap_C|GetDirectionArrow (Variables|/Game/Widget/HUDWidget.HUDWidget_C|GetMiniMap _mainwidget)) (select (> (Variables|Default|GetCurrentDistance) (Variables|Default|GetShowDirectionArrowAmount)) "HitTestInvisible" "Hidden"))
    (else
      (Variables|Default|SetCurrentGoalActor 0)
      (Widget|SetVisibility (Variables|/Game/Widget/HUDWidget.HUDWidget_C|GetDistanceBorder (Variables|Default|GetMainWidget)) "Hidden"))))

(event Custom|OnPlayerMove
  (Utilities|IsValid (Variables|Default|GetCurrentGoalActor)
    (:Is%20Valid
      (bind _output_get (Variables|Default|SetCurrentDistance (CallFunction|DistancetoGoal)))
      (Rendering|Components|TextRender|SetText (Variables|/Game/Widget/HUDWidget.HUDWidget_C|GetDistanceText (Variables|Default|GetMainWidget)) (Utilities|Text|ToText(Integer) _output_get false false))
      (Math|Integer|CompareInt (Variables|Default|GetCurrentDistance) (Variables|Default|GetShowDirectionArrowAmount)
        (:>
          _)
        (:==
          _)
        (:<
          (Utilities|FlowControl|DoOnce false :!label _label
            (:Completed
              (Widget|SetVisibility (Variables|/Game/Widget/MiniMap.MiniMap_C|GetDirectionArrow (Variables|/Game/Widget/HUDWidget.HUDWidget_C|GetMiniMap (Variables|Default|GetMainWidget))) "Hidden")
              (goto _label_2 Reset)))))
      (CallFunction|UpdateDirectionArrow)
      (Utilities|FlowControl|DoOnce false :!label _label_2
        (:Completed
          (Widget|SetVisibility (Variables|/Game/Widget/MiniMap.MiniMap_C|GetDirectionArrow (Variables|/Game/Widget/HUDWidget.HUDWidget_C|GetMiniMap (Variables|Default|GetMainWidget))) "HitTestInvisible")
          (goto _label Reset))))))

(event EventBeginPlay)

(event Collision|EventActorBeginOverlap
  (params (OtherActor :type Actor%20Object%20Reference)))

(event EventTick
  (params (DeltaSeconds :type Float%20%28single-precision%29)))

(fn ConstructionScript)

(fn SelectNewQuest
  (params (Quest :type BP%20Master%20Quest%20Object%20Reference) (SubGoal :type Sub%20Goal%20Widget%20Object%20Reference))
  (Utilities|IsValid (Variables|Default|GetCurrentQuest)
    (:Is%20Valid
      (Widget|SetIsEnabled (Variables|/Game/Widget/QuestWidget.QuestWidget_C|GetQuestName (Variables|/Game/Blueprints/Actors/QuestActors/BP_MasterQuest.BP_MasterQuest_C|GetQuestWidget (Variables|Default|GetCurrentQuest))) false)
      (Default|SelectSubGoal (Variables|/Game/Blueprints/Actors/QuestActors/BP_MasterQuest.BP_MasterQuest_C|GetQuestWidget (Variables|Default|GetCurrentQuest))))
    (:Is%20Not%20Valid
      _))
  (bind _output_get (Variables|Default|SetCurrentQuest Quest))
  (Default|OnQuestSelected (Variables|/Game/Blueprints/Actors/QuestActors/BP_MasterQuest.BP_MasterQuest_C|GetQuestWidget _output_get) SubGoal)
  (return))

(fn AddNewQuest
  (params (QuestClass :type BP%20Master%20Quest%20Class%20Reference) (DirectlyStart :type Boolean))
  (LocalVariables|SetlocalClass QuestClass)
  (LocalVariables|SetStart DirectlyStart)
  (if (and (Utilities|IsValidClass QuestClass) (not (Utilities|Array|ContainsItem (Variables|Default|GetAllQuestClasses) QuestClass)))
    (Utilities|Array|Add (Variables|Default|GetAllQuestClasses) (LocalVariables|GetlocalClass))
    (bind _returnvalue (Game|SpawnActorfromClass (LocalVariables|GetlocalClass) (Math|Transform|MakeTransform "0, 0, 0" "0, 0, 0" "1,1,1") "AlwaysSpawn" 0 0))
    (bind _output_get (LocalVariables|SetlocalQuestActor _returnvalue))
    (Utilities|Array|Add (Variables|Default|GetQuestActors) _output_get)
    (Default|SetupStartingGoals (LocalVariables|GetlocalQuestActor))
    (bind _widget (Default|AddQuesttoList (Variables|Default|GetMainWidget) (LocalVariables|GetlocalQuestActor)))
    (bind _output_get_2 (Variables|/Game/Blueprints/Actors/QuestActors/BP_MasterQuest.BP_MasterQuest_C|SetQuestWidget (LocalVariables|GetlocalQuestActor) _widget))
    (Default|UpdateQuest _output_get_2)
    (if (or (LocalVariables|GetStart) (<= (Utilities|Array|Length (Variables|Default|GetQuestActors)) 1))
      (CallFunction|SelectNewQuest (LocalVariables|GetlocalQuestActor) (Utilities|Array|Get(acopy) (Variables|/Game/Widget/QuestWidget.QuestWidget_C|GetSubGoalWidget (Variables|/Game/Blueprints/Actors/QuestActors/BP_MasterQuest.BP_MasterQuest_C|GetQuestWidget (LocalVariables|GetlocalQuestActor))))))
    (return true)
    (else
      (return false))))

(fn DistancetoGoal
  (bind _thirdpersonchar (Variables|Default|GetThirdPersonChar))
  (bind _currentgoalactor (Variables|Default|GetCurrentGoalActor))
  (bind _returnvalue (Transformation|GetActorLocation _thirdpersonchar))
  (bind _returnvalue_2 (Transformation|GetActorLocation _currentgoalactor))
  (return (Math|Float|Round (/ (Math|Vector|VectorLength (- (Math|Vector|MakeVector (.x _returnvalue) (.y _returnvalue) 0.0) (Math|Vector|MakeVector (.x _returnvalue_2) (.y _returnvalue_2) 0.0))) 1e+02))))

(fn UpdateDirectionArrow
  (Class|Widget|SetRenderTransformAngle (Variables|/Game/Widget/MiniMap.MiniMap_C|GetDirectionArrow (Variables|/Game/Widget/HUDWidget.HUDWidget_C|GetMiniMap (Variables|Default|GetMainWidget))) (.Yaw (Math|Rotator|BreakRotator (Math|Rotator|FindLookatRotation (Transformation|GetActorLocation (Variables|Default|GetThirdPersonChar)) (Transformation|GetActorLocation (Variables|Default|GetCurrentGoalActor))))))
  (return))