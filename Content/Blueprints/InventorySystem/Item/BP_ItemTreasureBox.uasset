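; BP_ItemTreasureBox is an inventory item that works as a treasure box, trading itself for jewelry when used.
; Its onUsed event removes one unit at its own inventory index, adds one earring, necklace and ring item to the same Inventory, then destroys the actor.
; The contents are fixed in the graph, with no randomization or check on whether the additions succeed.
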(event EventBeginPlay
  (|CallParentFunction) ; 지금 이 노드는 비활성 상태입니다. \n핀을 끌어서 다른 노드를 연결하면 활성화됩니다.
)

(event Collision|EventActorBeginOverlap
  (params (OtherActor :type Actor%20Object%20Reference))
  (|CallParentFunction OtherActor) ; 지금 이 노드는 비활성 상태입니다. \n핀을 끌어서 다른 노드를 연결하면 활성화됩니다.
)

(event EventTick
  (params (DeltaSeconds :type Float%20%28single-precision%29))
  (|CallParentFunction DeltaSeconds) ; 지금 이 노드는 비활성 상태입니다. \n핀을 끌어서 다른 노드를 연결하면 활성화됩니다.
)

(event EventEventonUsed
  (bind _inventory (Variables|Default|GetInventory))
  (Default|RemoveItematIndex (Variables|Default|GetInventory) (Variables|Default|GetIndex) 1)
  (Default|AddItem _inventory "/Game/Blueprints/InventorySystem/Item/BP_ItemEaring.BP_ItemEaring_C" 1)
  (Default|AddItem _inventory "/Game/Blueprints/InventorySystem/Item/BP_ItemNeckless.BP_ItemNeckless_C" 1)
  (Default|AddItem _inventory "/Game/Blueprints/InventorySystem/Item/BP_ItemRing.BP_ItemRing_C" 1)
  (Actor|DestroyActor))

(fn ConstructionScript
  (|CallParentFunction))